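; Base enemy character that exposes its patrol route, mesh and movement speed, likely for its AI to drive.
; An event spawns a hammer, attaches it to the right-hand socket and flags the enemy as wielding a weapon.
; Movement speed is set from discrete gait states, idle through running.
; PawnSensing, marked as old, sets the AI blackboard's player-seen flag on sighting the player.
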(event OnSeePawn(PawnSensing)
  (params (Pawn :type Pawn%20Object%20Reference))
  ;[0.15 0.15 0.15 0.5] Old sensing
  (Utilities|Casting|CastToBP_Player Pawn)
  (AI|Components|Blackboard|SetValueasBool (AI|GetBlackboard (AI|GetAIController self)) (Utilities|Name|MakeLiteralName "Player_seen") true))

(event Custom|Wield%20weapon
  ;[0.15 0.15 0.15 0.5] Wield weapon
  (bind _returnvalue (Game|SpawnActorfromClass "/Game/Assets/Weapons/Round_home_hammer/BP_Hammer.BP_Hammer_C" (Transformation|GetActorTransform) "Undefined" "MultiplyWithRoot" 0 0))
  (Transformation|AttachComponentToComponent _returnvalue (Variables|Character|GetMesh) "hand_r_Socket" "SnapToTarget" "SnapToTarget" "SnapToTarget" true)
  (Variables|Default|SetIs_Wielding_Weapon true))

(event EventBeginPlay)

(event Collision|EventActorBeginOverlap
  (params (OtherActor :type Actor%20Object%20Reference)))

(event EventTick
  (params (DeltaSeconds :type Float%20%28single-precision%29)))

(fn ConstructionScript)

(fn GetPatrolRoute
  (return (Variables|AI|GetPatrol_Route)))

(fn GetSkeletalMesh
  (return (Variables|Character|GetMesh)))

(fn SetMovementSpeed
  (params (Speed :type AI_Movement_Speed_E%20Enum :default "NewEnumerator0"))
  (Variables|/Script/Engine.CharacterMovementComponent|SetMaxWalkSpeed (Variables|Character|GetCharacterMovement) (Utilities|Select :Index Speed :NewEnumerator0 0.0 :NewEnumerator1 8e+01 :NewEnumerator3 2e+02 :NewEnumerator2 5e+02))
  (return 0.0))