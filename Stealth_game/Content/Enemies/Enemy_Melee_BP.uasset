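; Enemy_Melee_BP is a melee enemy that detects the player and can arm itself with a hammer.
; When PawnSensing sees a BP_Player, it sets the Player_seen blackboard key on its AI controller.
; The Wieldweapon event spawns a BP_Hammer, attaches it to the mesh's right-hand socket and flags the enemy as wielding a weapon.
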(event OnSeePawn(PawnSensing)
  (params (Pawn :type Pawn%20Object%20Reference))
  (Utilities|Casting|CastToBP_Player Pawn)
  (AI|Components|Blackboard|SetValueasBool (AI|GetBlackboard (AI|GetAIController self)) (Utilities|Name|MakeLiteralName "Player_seen") true))

(event Custom|Wield%20weapon
  (bind _returnvalue (Game|SpawnActorfromClass "/Game/Assets/Weapons/Round_home_hammer/BP_Hammer.BP_Hammer_C" (Transformation|GetActorTransform) "Undefined" "MultiplyWithRoot" 0 0))
  (Transformation|AttachComponentToComponent _returnvalue (Variables|Character|GetMesh) "hand_r_Socket" "SnapToTarget" "SnapToTarget" "SnapToTarget" true)
  (Variables|Default|SetIs_Wielding_Weapon true))

(event EventBeginPlay)

(event Collision|EventActorBeginOverlap
  (params (OtherActor :type Actor%20Object%20Reference)))

(event EventTick
  (params (DeltaSeconds :type Float%20%28single-precision%29)))

(fn ConstructionScript)